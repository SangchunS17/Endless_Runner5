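; BP_Immune is an item that grants the Jumper player character immunity when used.
; Tick polls the Used flag: the first use creates a SlotItembarUsed widget, sets Immune and starts its cast, while later uses only make the widget visible.
; When Used is false, Immune clears once the character is not casting.
; ReduceCastTimeValue increments every tick while the item level is a multiple of five.
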(event EventBeginPlay
  (|CallParentFunction) ; This node is disabled and will not be called.\nDrag off pins to build functionality.
)

(event Collision|EventActorBeginOverlap
  (params (OtherActor :type Actor%20Object%20Reference))
  (|CallParentFunction OtherActor) ; This node is disabled and will not be called.\nDrag off pins to build functionality.
)

(event EventTick
  (params (DeltaSeconds :type Float%20%28single-precision%29))
  (|CallParentFunction DeltaSeconds)
  ;[1 1 1] Upgrade
  (if (== (Math|Integer|%(Integer) (.level (Variables|Default|GetItem_Detail)) 5) 0)
    (Math|Integer|IncrementInt (Variables|Default|GetReduceCastTimeValue)
      (:%20%20
        _)))
  (if (Variables|Default|GetUsed?)
    (if (== (Variables|Default|GetWidgetUI) 0)
      ;[1 1 1] Comment
      (bind _returnvalue (UserInterface|CreateWidget "/Game/UI/HotKey/SlotItemuse/SlotItembarUsed.SlotItembarUsed_C"))
      (bind _output_get (Variables|Default|SetWidgetUI _returnvalue))
      (UserInterface|Viewport|AddtoViewport _output_get 0)
      (Class|UserWidget|SetDesiredSizeinViewport _output_get "(X=60.000000,Y=60.000000)")
      (bind _output_get_2 (Variables|/Game/UI/HotKey/SlotItemuse/SlotItembarUsed.SlotItembarUsed_C|SetItem _output_get (Utilities|GetClass self)))
      (Variables|Default|SetUsed? false)
      (bind _asjumper_bp (Utilities|Casting|CastToJumper_BP (Game|GetPlayerCharacter 0)))
      (Variables|/Game/Blueprint/Chracter/Jumper_BP.Jumper_BP_C|SetImmune _asjumper_bp true)
      (Default|StartCast _output_get (Variables|/Game/UI/HotKey/SlotItemuse/SlotItembarUsed.SlotItembarUsed_C|GetSlotitmebar _output_get) _output_get_2)
      (else
        (Widget|SetVisibility (Variables|Default|GetWidgetUI) "Visible")))
    (else
      (bind _asjumper_bp_2 (Utilities|Casting|CastToJumper_BP (Game|GetPlayerCharacter 0)))
      (if (not (Variables|/Game/Blueprint/Chracter/Jumper_BP.Jumper_BP_C|GetCureentCasting _asjumper_bp_2))
        (Variables|/Game/Blueprint/Chracter/Jumper_BP.Jumper_BP_C|SetImmune _asjumper_bp_2 false)))))

(fn ConstructionScript
  (|CallParentFunction))