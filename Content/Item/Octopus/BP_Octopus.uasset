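; BP_Octopus is an octopus hazard item in the endless-run game that slows the player on contact.
; When Jumper_BP overlaps its mesh under the EndlessRun game mode, it adds an Effect_Octopus widget to the screen and lowers the character's max walk speed, clamped to a fixed range.
; It then hides the mesh and destroys itself, so it triggers only once.
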(event OnComponentBeginOverlap(StaticMesh)
  (params (OverlappedComponent :type Primitive%20Component%20Object%20Reference) (OtherActor :type Actor%20Object%20Reference) (OtherComp :type Primitive%20Component%20Object%20Reference) (OtherBodyIndex :type Integer) (bFromSweep :type Boolean) (SweepResult :type Hit%20Result%20Structure%20%28by%20ref%29))
  (bind _asjumper_bp (Utilities|Casting|CastToJumper_BP OtherActor))
  (Utilities|Casting|CastToEndlessRun (Game|GetGameMode))
  (bind _returnvalue (UserInterface|CreateWidget "/Game/UI/UsedItemUI/Effect_Octopus/Effect_Octopus.Effect_Octopus_C"))
  (UserInterface|Viewport|AddtoViewport _returnvalue 0)
  (Variables|/Script/Engine.CharacterMovementComponent|SetMaxWalkSpeed (Variables|/Script/Engine.Character|GetCharacterMovement _asjumper_bp) (Math|Float|Clamp(Float) (- (Variables|/Script/Engine.CharacterMovementComponent|GetMaxWalkSpeed (Variables|/Script/Engine.Character|GetCharacterMovement _asjumper_bp)) 1e+02) 6e+02 2e+03))
  (Rendering|SetVisibility (Variables|Default|GetStaticMesh) false false)
  (Actor|DestroyActor))

(fn ConstructionScript
  (|CallParentFunction))