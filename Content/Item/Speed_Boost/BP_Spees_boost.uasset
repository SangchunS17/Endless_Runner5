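; Speed boost pickup actor that grants the Jumper_BP character a movement speed buff when it overlaps the mesh.
; On overlap it hides the mesh without destroying the actor or disabling collision.
; If no buff is active, it flags one, raises clamped max walk speed and sets DelayTimeDestroy on the character.
; It starts the SpdBuff cast on player zero's UI even when the buff is already active.
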(event OnComponentBeginOverlap(StaticMesh)
  (params (OverlappedComponent :type Primitive%20Component%20Object%20Reference) (OtherActor :type Actor%20Object%20Reference) (OtherComp :type Primitive%20Component%20Object%20Reference) (OtherBodyIndex :type Integer) (bFromSweep :type Boolean) (SweepResult :type Hit%20Result%20Structure%20%28by%20ref%29))
  (bind _asjumper_bp (Utilities|Casting|CastToJumper_BP OtherActor))
  (Rendering|SetVisibility (Variables|Default|GetStaticMesh) false false)
  (bind _asjumper_bp_2 (Utilities|Casting|CastToJumper_BP (Game|GetPlayerCharacter 0)))
  (if (Variables|/Game/Blueprint/Chracter/Jumper_BP.Jumper_BP_C|Getspd_buff_active _asjumper_bp)
    _
    (else
      (Variables|/Game/Blueprint/Chracter/Jumper_BP.Jumper_BP_C|Setspd_buff_active _asjumper_bp true)
      (Variables|/Script/Engine.CharacterMovementComponent|SetMaxWalkSpeed (Variables|/Script/Engine.Character|GetCharacterMovement _asjumper_bp) (Math|Float|Clamp(Float) (+ (Variables|/Script/Engine.CharacterMovementComponent|GetMaxWalkSpeed (Variables|/Script/Engine.Character|GetCharacterMovement _asjumper_bp)) 5e+02 0.0) 6e+02 2e+03))
      (Variables|/Game/Blueprint/Chracter/Jumper_BP.Jumper_BP_C|SetDelayTimeDestroy _asjumper_bp 1e+01)))
  (Default|StartCast (Variables|/Game/UI/BaseUI/BaseUI_Runner.BaseUI_Runner_C|GetSpd_buff (Variables|/Game/Blueprint/Chracter/Jumper_BP.Jumper_BP_C|GetBaseUI _asjumper_bp_2)) (Variables|/Game/UI/BaseUI/BaseUI_Runner.BaseUI_Runner_C|GetSpd_buff (Variables|/Game/Blueprint/Chracter/Jumper_BP.Jumper_BP_C|GetBaseUI _asjumper_bp_2))))

(event EventBeginPlay
  (|CallParentFunction) ; This node is disabled and will not be called.\nDrag off pins to build functionality.
)

(event Collision|EventActorBeginOverlap
  (params (OtherActor :type Actor%20Object%20Reference))
  (|CallParentFunction OtherActor) ; This node is disabled and will not be called.\nDrag off pins to build functionality.
)

(fn ConstructionScript
  (|CallParentFunction))