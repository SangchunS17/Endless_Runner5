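; BP_SlowMove is an item that, when used, changes the player's max walk speed to a fixed value, as a slow-move effect.
; Tick polls the Used flag and, on first use, creates a SlotItembarUsed widget, saves the Jumper_BP speed on the character, applies the new speed and starts the widget's cast.
; While Used is false, Tick restores the saved speed whenever the player's CureentCasting flag is off.
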(event EventBeginPlay
  (|CallParentFunction) ; This node is disabled and will not be called.\nDrag off pins to build functionality.
)

(event Collision|EventActorBeginOverlap
  (params (OtherActor :type Actor%20Object%20Reference))
  (|CallParentFunction OtherActor) ; This node is disabled and will not be called.\nDrag off pins to build functionality.
)

(event EventTick
  (params (DeltaSeconds :type Float%20%28single-precision%29))
  (|CallParentFunction DeltaSeconds)
  (if (Variables|Default|GetUsed?)
    (if (== (Variables|Default|GetWidgetSlot) 0)
      (bind _returnvalue (UserInterface|CreateWidget "/Game/UI/HotKey/SlotItemuse/SlotItembarUsed.SlotItembarUsed_C"))
      (bind _output_get (Variables|Default|SetWidgetSlot _returnvalue))
      (UserInterface|Viewport|AddtoViewport _output_get 0)
      (Class|UserWidget|SetDesiredSizeinViewport _output_get "(X=60.000000,Y=60.000000)")
      (bind _output_get_2 (Variables|/Game/UI/HotKey/SlotItemuse/SlotItembarUsed.SlotItembarUsed_C|SetItem _output_get (Utilities|GetClass self)))
      (Variables|Default|SetUsed? false)
      (bind _asjumper_bp (Utilities|Casting|CastToJumper_BP (Game|GetPlayerCharacter 0)))
      (Variables|/Game/Blueprint/Chracter/Jumper_BP.Jumper_BP_C|SetCurrenttMaxWalkSpeed _asjumper_bp (Variables|/Script/Engine.CharacterMovementComponent|GetMaxWalkSpeed (Variables|/Script/Engine.Character|GetCharacterMovement _asjumper_bp)))
      (Variables|/Script/Engine.CharacterMovementComponent|SetMaxWalkSpeed (Variables|/Script/Engine.Character|GetCharacterMovement _asjumper_bp) 4e+02)
      (Default|StartCast _output_get (Variables|/Game/UI/HotKey/SlotItemuse/SlotItembarUsed.SlotItembarUsed_C|GetSlotitmebar _output_get) _output_get_2)
      (else
        (Widget|SetVisibility (Variables|Default|GetWidgetSlot) "Visible")))
    (else
      (bind _asjumper_bp_2 (Utilities|Casting|CastToJumper_BP (Game|GetPlayerCharacter 0)))
      (if (not (Variables|/Game/Blueprint/Chracter/Jumper_BP.Jumper_BP_C|GetCureentCasting _asjumper_bp_2))
        (Variables|/Script/Engine.CharacterMovementComponent|SetMaxWalkSpeed (Variables|/Script/Engine.Character|GetCharacterMovement _asjumper_bp_2) (Variables|/Game/Blueprint/Chracter/Jumper_BP.Jumper_BP_C|GetCurrenttMaxWalkSpeed _asjumper_bp_2))))))

(fn ConstructionScript
  (|CallParentFunction))