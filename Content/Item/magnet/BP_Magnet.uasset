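; BP_Magnet is a magnet pickup for the endless run game, collected when Jumper_BP overlaps its static mesh.
; If the EndlessRun game mode reports the magnet inactive, it calls StartCast on the Magnet element of the player's BaseUI and hides the mesh.
; The actor only reads MagnetActive and contains no attraction logic or destroy call of its own.
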(event OnComponentBeginOverlap(StaticMesh)
  (params (OverlappedComponent :type Primitive%20Component%20Object%20Reference) (OtherActor :type Actor%20Object%20Reference) (OtherComp :type Primitive%20Component%20Object%20Reference) (OtherBodyIndex :type Integer) (bFromSweep :type Boolean) (SweepResult :type Hit%20Result%20Structure%20%28by%20ref%29))
  (bind _asjumper_bp (Utilities|Casting|CastToJumper_BP OtherActor))
  (bind _asendless_run (Utilities|Casting|CastToEndlessRun (Game|GetGameMode)))
  (if (not (Variables|/Game/Blueprint/GameMode/EndlessRun.EndlessRun_C|GetMagnetActive _asendless_run))
    (Default|StartCast (Variables|/Game/UI/BaseUI/BaseUI_Runner.BaseUI_Runner_C|GetMagnet (Variables|/Game/Blueprint/Chracter/Jumper_BP.Jumper_BP_C|GetBaseUI _asjumper_bp)) (Variables|/Game/UI/BaseUI/BaseUI_Runner.BaseUI_Runner_C|GetMagnet (Variables|/Game/Blueprint/Chracter/Jumper_BP.Jumper_BP_C|GetBaseUI _asjumper_bp)))
    (Rendering|SetVisibility (Variables|Default|GetStaticMesh) false false)))

(event EventBeginPlay
  (|CallParentFunction) ; This node is disabled and will not be called.\nDrag off pins to build functionality.
)

(event Collision|EventActorBeginOverlap
  (params (OtherActor :type Actor%20Object%20Reference))
  (|CallParentFunction OtherActor) ; This node is disabled and will not be called.\nDrag off pins to build functionality.
)

(event EventTick
  (params (DeltaSeconds :type Float%20%28single-precision%29))
  (|CallParentFunction DeltaSeconds) ; This node is disabled and will not be called.\nDrag off pins to build functionality.
)

(fn ConstructionScript
  (|CallParentFunction))