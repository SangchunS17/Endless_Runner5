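; Obstacle block that counts hits on the player's Jumper_BP and kills it when the count reaches two.
; Each Cube overlap increments the jumper's ColliderObstacle counter, so the tally lives on the player and the obstacle calls Death.
; SetBoxCollision toggles a given object's collision and visibility together.
; SpawnEnv adds two child actor components on opposite sides, rotated to opposite yaws; two further placements are unwired.
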(event OnComponentBeginOverlap(Cube)
  (params (OverlappedComponent :type Primitive%20Component%20Object%20Reference) (OtherActor :type Actor%20Object%20Reference) (OtherComp :type Primitive%20Component%20Object%20Reference) (OtherBodyIndex :type Integer) (bFromSweep :type Boolean) (SweepResult :type Hit%20Result%20Structure%20%28by%20ref%29))
  (bind _asjumper_bp (Utilities|Casting|CastToJumper_BP OtherActor))
  (Math|Integer|IncrementInt (Variables|/Game/Blueprint/Chracter/Jumper_BP.Jumper_BP_C|GetColliderObstacle _asjumper_bp)
    (:%20%20
      (if (== (Variables|/Game/Blueprint/Chracter/Jumper_BP.Jumper_BP_C|GetColliderObstacle _asjumper_bp) 2)
        (Default|Death _asjumper_bp)))))

(event EventBeginPlay)

(fn ConstructionScript)

(fn SetBoxCollision
  (params (Enable :type Boolean) (Object :type Primitive%20Component%20Object%20Reference))
  (if Enable
    (Collision|SetCollisionEnabled Object "QueryAndPhysics")
    (Rendering|SetVisibility Object true false)
    (else
      (Collision|SetCollisionEnabled Object "NoCollision")
      (Rendering|SetVisibility Object false false))))

(fn SpawnEnv
  (Utilities|FlowControl|Sequence
    (:then_0
      (AddComponent|AddChildActorComponent false (Math|Transform|MakeTransform "-440.000000,290.000000,81.000000" "0.000000,90.000000,0.000000" "1.000000,1.000000,1.000000")))
    (:then_1
      (AddComponent|AddChildActorComponent false (Math|Transform|MakeTransform "440.000000,310.000000,81.000000" "0.000000,-90.000000,0.000000" "1.000000,1.000000,1.000000")))))