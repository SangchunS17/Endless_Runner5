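; Starting level block for the jumper game that dresses itself with environment pieces and removes itself shortly after play begins.
; On BeginPlay, SpawnEnv adds child actors in mirrored pairs on both sides, then after a delay the block destroys itself unless the player is dead.
; Overlapping the water collision calls Death on Jumper_BP.
; A SetBoxCollision helper toggles an object's collision and visibility together, but is not called here.
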(event OnComponentBeginOverlap(Wather_collision)
  (params (OverlappedComponent :type Primitive%20Component%20Object%20Reference) (OtherActor :type Actor%20Object%20Reference) (OtherComp :type Primitive%20Component%20Object%20Reference) (OtherBodyIndex :type Integer) (bFromSweep :type Boolean) (SweepResult :type Hit%20Result%20Structure%20%28by%20ref%29))
  (bind _asjumper_bp (Utilities|Casting|CastToJumper_BP OtherActor))
  (Default|Death _asjumper_bp))

(event EventBeginPlay
  (CallFunction|SpawnEnv)
  (Utilities|FlowControl|Delay 5.0)
  (bind _asjumper_bp (Utilities|Casting|CastToJumper_BP (Game|GetPlayerCharacter 0)))
  (if (not (Variables|/Game/Blueprint/Chracter/Jumper_BP.Jumper_BP_C|GetIsDeath _asjumper_bp))
    (Actor|DestroyActor)))

(fn ConstructionScript)

(fn SetBoxCollision
  (params (Enable :type Boolean) (Object :type Primitive%20Component%20Object%20Reference))
  (if Enable
    (Collision|SetCollisionEnabled Object "QueryAndPhysics")
    (Rendering|SetVisibility Object true false)
    (else
      (Collision|SetCollisionEnabled Object "NoCollision")
      (Rendering|SetVisibility Object false false))))

(fn SpawnEnv
  (Utilities|FlowControl|Sequence
    (:then_0
      (AddComponent|AddChildActorComponent false (Math|Transform|MakeTransform "-430.000000,0.000000,81.000000" "0.000000,89.000000,0.000000" "1.000000,1.000000,1.000000"))
      (AddComponent|AddChildActorComponent false (Math|Transform|MakeTransform "430.000000,0.000000,81.000000" "0.000000,-89.000000,0.000000" "1.000000,1.000000,1.000000")))
    (:then_1
      (AddComponent|AddChildActorComponent false (Math|Transform|MakeTransform "-430.000000,0.000000,81.000000" "0.000000,89.000000,0.000000" "1.000000,1.000000,1.000000"))
      (AddComponent|AddChildActorComponent false (Math|Transform|MakeTransform "430.000000,0.000000,81.000000" "0.000000,-89.000000,0.000000" "1.000000,1.000000,1.000000")))))