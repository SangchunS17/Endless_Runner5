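; Endless-runner track block with three rock lanes over water, which kills the Jumper on contact.
; BeginPlay randomly enables lanes, keeping at least one (all during speed or three-way buffs), then randomly spawns coins, power-ups, octopuses or obstacles on them.
; Entering EnterBox adds score, spawns the next BlockM2 at the Arrow, nudges up max speed and adds side scenery.
; The block then destroys itself after a speed-scaled delay unless the player is dead.
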(event OnComponentBeginOverlap(EnterBox)
  (params (OverlappedComponent :type Primitive%20Component%20Object%20Reference) (OtherActor :type Actor%20Object%20Reference) (OtherComp :type Primitive%20Component%20Object%20Reference) (OtherBodyIndex :type Integer) (bFromSweep :type Boolean) (SweepResult :type Hit%20Result%20Structure%20%28by%20ref%29))
  (bind _asjumper_bp (Utilities|Casting|CastToJumper_BP OtherActor))
  (Math|Integer|IncrementInt (Variables|/Game/Blueprint/Chracter/Jumper_BP.Jumper_BP_C|GetScore _asjumper_bp)
    (:%20%20
      (Game|SpawnActorfromClass "BlockM2_C" (Transformation|GetWorldTransform (Variables|Default|GetArrow)) "Undefined" 0 0)
      (bind _asjumper_bp_2 (Utilities|Casting|CastToJumper_BP (Game|GetPlayerCharacter 0)))
      (Variables|/Script/Engine.CharacterMovementComponent|SetMaxWalkSpeed (Variables|/Script/Engine.Character|GetCharacterMovement _asjumper_bp_2) (Math|Float|Clamp(Float) (* (Variables|/Script/Engine.CharacterMovementComponent|GetMaxWalkSpeed (Variables|/Script/Engine.Character|GetCharacterMovement _asjumper_bp_2)) 1.0001) (Variables|/Script/Engine.CharacterMovementComponent|GetMaxWalkSpeed (Variables|/Script/Engine.Character|GetCharacterMovement _asjumper_bp_2)) 2e+03))
      (bind _asjumper_bp_3 (Utilities|Casting|CastToJumper_BP (Game|GetPlayerCharacter 0)))
      (CallFunction|RandomEnv)
      (Utilities|FlowControl|Delay 0.2)
      (Utilities|FlowControl|Delay (/ (* (Variables|/Game/Blueprint/Chracter/Jumper_BP.Jumper_BP_C|GetCurrenttMaxWalkSpeed _asjumper_bp_3) (Variables|/Game/Blueprint/Chracter/Jumper_BP.Jumper_BP_C|GetDelayTimeDestroy _asjumper_bp_3)) (Variables|/Script/Engine.CharacterMovementComponent|GetMaxWalkSpeed (Variables|/Script/Engine.Character|GetCharacterMovement _asjumper_bp_3))))
      (bind _asjumper_bp_4 (Utilities|Casting|CastToJumper_BP (Game|GetPlayerCharacter 0)))
      (if (not (Variables|/Game/Blueprint/Chracter/Jumper_BP.Jumper_BP_C|GetIsDeath _asjumper_bp_4))
        (Actor|DestroyActor)))))

(event OnComponentBeginOverlap(Wather)
  (params (OverlappedComponent :type Primitive%20Component%20Object%20Reference) (OtherActor :type Actor%20Object%20Reference) (OtherComp :type Primitive%20Component%20Object%20Reference) (OtherBodyIndex :type Integer) (bFromSweep :type Boolean) (SweepResult :type Hit%20Result%20Structure%20%28by%20ref%29))
  (bind _asjumper_bp (Utilities|Casting|CastToJumper_BP OtherActor))
  (Variables|/Game/Blueprint/Chracter/Jumper_BP.Jumper_BP_C|SetIsWatering _asjumper_bp true)
  (Default|Death _asjumper_bp)
  (if (Variables|/Game/Blueprint/Chracter/Jumper_BP.Jumper_BP_C|GetIsDeath _asjumper_bp)
    (Components|MoveComponentTo (Variables|Default|GetBox) "0.000000,0.000000,-80.000000" "0, 0, 0" false false 0.25 false)
    (Physics|SetSimulatePhysics (Variables|/Script/Engine.Character|GetMesh _asjumper_bp) false)
    (Components|Animation|PlayAnimation (Variables|/Script/Engine.Character|GetMesh _asjumper_bp) "/Game/Characters/Mannequins/Animations/Quinn/Floating_Anim_mixamo_com.Floating_Anim_mixamo_com" true)))

(event EventBeginPlay
  (bind _asjumper_bp (Utilities|Casting|CastToJumper_BP (Game|GetPlayerCharacter 0)))
  (if (or (Variables|/Game/Blueprint/Chracter/Jumper_BP.Jumper_BP_C|Getspd_buff_active _asjumper_bp) (Variables|/Game/Blueprint/Chracter/Jumper_BP.Jumper_BP_C|GetThreeWay _asjumper_bp))
    (Variables|Default|SetWay1_Enable true)
    (Variables|Default|SetWay2_Enable true)
    (Variables|Default|SetWay3_Enable true)
    (else
      (Variables|Default|SetWay1_Enable (Math|Random|RandomBool))
      (Variables|Default|SetWay2_Enable (Math|Random|RandomBool))
      (Variables|Default|SetWay3_Enable (Math|Random|RandomBool))))
  (CallFunction|SetBoxCollision (Variables|Default|GetWay1_Enable) (Variables|Default|GetRock1))
  (CallFunction|SetBoxCollision (Variables|Default|GetWay2_Enable) (Variables|Default|GetRock2))
  (CallFunction|SetBoxCollision (Variables|Default|GetWay3_Enable) (Variables|Default|GetRock3))
  (if (Math|Boolean|ANDBoolean (not (Variables|Default|GetWay1_Enable)) (not (Variables|Default|GetWay2_Enable)) (not (Variables|Default|GetWay3_Enable)))
    (Variables|Default|SetRandomWay (Math|Random|RandomIntegerinRange 1 3))
    (switch int (Variables|Default|GetRandomWay)
      (:1
        (CallFunction|SetBoxCollision true (Variables|Default|GetRock1))
        (Variables|Default|SetWay1_Enable true))
      (:2
        (CallFunction|SetBoxCollision true (Variables|Default|GetRock2))
        (Variables|Default|SetWay2_Enable true))
      (:3
        (CallFunction|SetBoxCollision true (Variables|Default|GetRock3))
        (Variables|Default|SetWay3_Enable true))))
  ;[1 1 1] Random lane and item
  (bind _returnvalue (CallFunction|RandomLane (Variables|Default|GetWay1_Enable)))
  (if _returnvalue
    (CallFunction|RandomSpawnItem (Variables|Default|GetRock1)))
  (bind _returnvalue_2 (CallFunction|RandomLane (Variables|Default|GetWay2_Enable)))
  (if _returnvalue_2
    (CallFunction|RandomSpawnItem (Variables|Default|GetRock2)))
  (bind _returnvalue_3 (CallFunction|RandomLane (Variables|Default|GetWay3_Enable)))
  (if _returnvalue_3
    (CallFunction|RandomSpawnItem (Variables|Default|GetRock3))))

(event Collision|EventActorBeginOverlap
  (params (OtherActor :type Actor%20Object%20Reference)))

(event EventTick
  (params (DeltaSeconds :type Float%20%28single-precision%29)))

(fn ConstructionScript)

(fn SetBoxCollision
  (params (Enable :type Boolean) (Object :type Primitive%20Component%20Object%20Reference))
  (if Enable
    (Collision|SetCollisionEnabled Object "QueryAndPhysics")
    (Rendering|SetVisibility Object true false)
    (else
      (Collision|SetCollisionEnabled Object "NoCollision")
      (Rendering|SetVisibility Object false false))))

(fn RandomSpawnItem
  (params (Rock :type Static%20Mesh%20Component%20Object%20Reference))
  (bind _returnvalue (Math|Random|RandomFloatinRange 0.0 1.0))
  (if (Math|Float|InRange(Float) _returnvalue 0.0 0.5)
    (for _index (range 0 (Math|Random|RandomIntegerinRange 0 4))
      (bind _ascoin (Utilities|Casting|CastToCoinClass "/Game/Item/Coin/Coin.Coin_C"))
      (CallFunction|SpawnItem _ascoin Rock (Math|Conversions|ToFloat(Integer) (* _index 50)) 0.0))
    (elif (Math|Float|InRange(Float) _returnvalue 0.5 0.58)
      (bind _asbp_magnet (Utilities|Casting|CastToBP_MagnetClass "/Game/Item/magnet/BP_Magnet.BP_Magnet_C"))
      (CallFunction|SpawnItem _asbp_magnet Rock 0.0 0.0)
      (elif (Math|Float|InRange(Float) _returnvalue 0.58 0.62)
        (bind _asbp_multiply_two (Utilities|Casting|CastToBP_MultiplyTwoClass "/Game/Item/MultiplyTwo/BP_MultiplyTwo.BP_MultiplyTwo_C"))
        (CallFunction|SpawnItem _asbp_multiply_two Rock 0.0 0.0)
        (elif (Math|Float|InRange(Float) _returnvalue 0.62 0.7)
          (bind _asbp_spees_boost (Utilities|Casting|CastToBP_Spees_boostClass "/Game/Item/Speed_Boost/BP_Spees_boost.BP_Spees_boost_C"))
          (CallFunction|SpawnItem _asbp_spees_boost Rock 0.0 0.0)
          (elif (Math|Float|InRange(Float) _returnvalue 0.7 1.0)
            (bind _asbp_octopus (Utilities|Casting|CastToBP_OctopusClass "/Game/Item/Octopus/BP_Octopus.BP_Octopus_C"))
            (CallFunction|SpawnItem _asbp_octopus Rock 0.0 0.0)
            (else
              (bind _asbp_obstacle (Utilities|Casting|CastToBP_obstacleClass "/Game/Blueprint/Block/BP_obstacle.BP_obstacle_C"))
              (CallFunction|SpawnItem _asbp_obstacle Rock 0.0 -45.0))))))))

(fn SpawnItem
  (params (ItemClass :type Actor%20Class%20Reference) (Target :type Scene%20Component%20Object%20Reference) (X :type Float%20%28double-precision%29) (Z :type Float%20%28double-precision%29))
  (Game|SpawnActorfromClass ItemClass (Math|Conversions|ToTransform(Vector) (+ (Transformation|GetWorldLocation Target) (Math|Vector|MakeVector X 0.0 (+ Z 1.6e+02)))) "Undefined" 0 0))

(fn RandomLane
  (params (Way :type Boolean))
  (bind _returnvalue (Math|Random|RandomBool))
  (bind _returnvalue_2 (and Way _returnvalue))
  (if _returnvalue_2
    (return _returnvalue_2)))

(fn RandomEnv
  (if (Math|Integer|InRange(Integer) (Math|Random|RandomIntegerinRange 0 1) 0 0)
    (AddComponent|AddChildActorComponent false (Math|Transform|MakeTransform "-430.000000,0.000000,81.000000" "0.000000,89.000000,0.000000" "1.000000,1.000000,1.000000"))
    (AddComponent|AddChildActorComponent false (Math|Transform|MakeTransform "430.000000,0.000000,81.000000" "0.000000,-89.000000,0.000000" "1.000000,1.000000,1.000000"))
    (else
      (AddComponent|AddChildActorComponent false (Math|Transform|MakeTransform "-430.000000,0.000000,81.000000" "0.000000,89.000000,0.000000" "1.000000,1.000000,1.000000"))
      (AddComponent|AddChildActorComponent false (Math|Transform|MakeTransform "430.000000,0.000000,81.000000" "0.000000,-89.000000,0.000000" "1.000000,1.000000,1.000000")))))