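; Jumper character Blueprint, named as built on C++, that slides sideways between lanes.
; On BeginPlay it finds the Camera actor in the level and makes it player 0's view target.
; Each tick, if the actor's Y differs from CurentLane times JumpDistance, a short MoveComponentTo on the capsule eases it to that lane, passing current X and Z.
; The lane value is only read here, never set.
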(event EventBeginPlay
  (bind _returnvalue (Actor|GetActorOfClass "/Game/Blueprint/Camera/Camera.Camera_C"))
  (Game|Player|SetViewTargetwithBlend (Game|GetPlayerController 0) _returnvalue 0.0 "VTBlend_Linear" 0.0 false))

(event Collision|EventActorBeginOverlap
  (params (OtherActor :type Actor%20Object%20Reference)))

(event EventTick
  (params (DeltaSeconds :type Float%20%28single-precision%29))
  (bind _returnvalue (Transformation|GetActorLocation))
  (bind _curentlane (Variables|Default|GetCurentLane))
  (bind _jumpdistance (Variables|Default|GetJumpDistance))
  (bind _returnvalue_2 (* _curentlane _jumpdistance))
  (if (!= _returnvalue_2 (.y (Transformation|GetActorLocation)))
    (Components|MoveComponentTo (Variables|Default|GetCapsuleComponent) (Math|Vector|MakeVector (.x _returnvalue) _returnvalue_2 (.z _returnvalue)) "0, 0, 0" false false 0.1 false)))

(fn ConstructionScript)