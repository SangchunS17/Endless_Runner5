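; Player character for a lane-based endless runner that runs forward automatically, with the view set to a level camera.
; Tick adds forward input and slides the capsule to the current lane, which left/right jumps change, alongside double jump and downward slam.
; Q and E spawn items from saved slots, decrementing and saving inventory to the HighScoreData slot.
; Death, skipped when immune, disables movement, ragdolls outside water and shows Game Over.
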(event Custom|Death
  (bind _mesh (Variables|Character|GetMesh))
  (bind _charactermovement (Variables|Character|GetCharacterMovement))
  (if (not (Variables|Default|GetImmune))
    (Development|PrintString (Utilities|String|ToString(Integer) (Variables|Default|GetCoin)) true true "(R=0.000000,G=0.660000,B=1.000000,A=1.000000)" 2e+01)
    ;[1 1 1] Death
    (Variables|Default|SetIsDeath true)
    (Utilities|FlowControl|Delay 0.25)
    (if (Variables|Default|GetIsWatering)
      (Variables|/Script/Engine.CharacterMovementComponent|SetMaxWalkSpeed _charactermovement -5.0)
      (Pawn|Components|CharacterMovement|DisableMovement _charactermovement)
      (else
        (Pawn|Components|CharacterMovement|DisableMovement _charactermovement)
        (Collision|SetCollisionProfileName _mesh "Ragdoll" true :!class /Script/Engine.PrimitiveComponent)
        (Physics|SetSimulatePhysics _mesh true)))
    (bind _returnvalue (UserInterface|CreateWidget "/Game/UI/GameOver/GameOver.GameOver_C"))
    (UserInterface|Viewport|AddtoViewport _returnvalue 0)))

(event Collision|EventActorBeginOverlap
  (params (OtherActor :type Actor%20Object%20Reference)))

(event EventTick
  (params (DeltaSeconds :type Float%20%28single-precision%29))
  (bind _returnvalue (Transformation|GetActorLocation))
  (bind _currentlane (Variables|Default|GetCurrentLane))
  (bind _jumpdistance (Variables|Default|GetJumpDistance))
  (bind _returnvalue_2 (* _currentlane _jumpdistance))
  ;[1 1 1] Event trick to run / check state
  (Utilities|FlowControl|Sequence
    (:then_0
      (Pawn|Input|AddMovementInput (Class|PawnMovementComponent|GetPawnOwner (Variables|Character|GetCharacterMovement)) (Math|Vector|MakeVector 1.0 0.0 0.0) 1.0 false))
    (:then_1
      (if (AI|Components|NavMovement|IsFalling (Variables|Character|GetCharacterMovement))
        (Variables|Default|SetIsInAir true)
        (CallFunction|SetPlayerDirection (Variables|Character|GetCharacterMovement))
        (else
          (Variables|Default|SetIsInAir false)
          (Variables|Default|SetCountJumpInAir 0))))
    (:then_2
      (if (!= _returnvalue_2 (.y (Transformation|GetActorLocation)))
        (Components|MoveComponentTo (Variables|Collision|GetCapsuleComponent) (Math|Vector|MakeVector (.x _returnvalue) _returnvalue_2 (.z _returnvalue)) "0, 0, 0" false false 0.1 false)))))

(event EventBeginPlay
  (bind _charactermovement (Variables|Character|GetCharacterMovement))
  ;[1 1 1] Set Defult Setting
  (Variables|/Script/Engine.CharacterMovementComponent|SetBrakingDecelerationFalling _charactermovement 1e+03)
  (Variables|/Script/Engine.CharacterMovementComponent|SetAirControl _charactermovement 1e+02)
  (Variables|/Script/Engine.CharacterMovementComponent|SetFallingLateralFriction _charactermovement 1e+03)
  (Variables|/Script/Engine.CharacterMovementComponent|SetbOrientRotationToMovement _charactermovement true)
  (Variables|/Script/Engine.CharacterMovementComponent|SetJumpZVelocity _charactermovement 5e+02)
  (Variables|Default|SetbUseControllerRotationYaw false)
  (bind _returnvalue (Actor|GetActorOfClass "/Game/Blueprint/Camera/Camera.Camera_C"))
  (Game|Player|SetViewTargetwithBlend (Game|GetPlayerController 0) _returnvalue 0.0 "VTBlend_Linear" 0.0 false)
  (Variables|Default|SetCurrenttMaxWalkSpeed (Variables|/Script/Engine.CharacterMovementComponent|GetMaxWalkSpeed _charactermovement))
  (bind _returnvalue_2 (SaveGame|DoesSaveGameExist "HighScoreData"))
  (if _returnvalue_2
    (bind _returnvalue_3 (SaveGame|LoadGamefromSlot "HighScoreData"))
    (bind _output_get (Variables|Default|SetSavegame _returnvalue_3))
    (bind _asendless_save_game (Utilities|Casting|CastToEndless_SaveGame _output_get))
    (Variables|Default|SetPlayerItem (Variables|/Game/Save/Endless_SaveGame.Endless_SaveGame_C|GetPlayerItem _asendless_save_game))
    (Development|PrintString "Save" true true "(R=0.000000,G=0.660000,B=1.000000,A=1.000000)" 1e+01)
    (Variables|Default|SetSlotItemUsed (Variables|/Game/Save/Endless_SaveGame.Endless_SaveGame_C|GetSlotItem _asendless_save_game))))

(event Input|ActionEvents|InputActionDoubleJump
  (params (Key :type Key%20Structure :default "None"))
  (bind _charactermovement (Variables|Character|GetCharacterMovement))
  (bind _returnvalue (Pawn|Components|CharacterMovement|GetLastUpdateVelocity _charactermovement))
  ;[1 1 1] Jump L/R
  (:Pressed
    (if (< (Variables|Default|GetCountJumpInAir) 2)
      (if (Variables|Default|GetIsInAir)
        (Variables|/Script/Engine.MovementComponent|SetVelocity (Variables|Character|GetCharacterMovement) (Math|Vector|MakeVector (.x _returnvalue) (.y _returnvalue) 4e+02))
        (Variables|Default|SetCountJumpInAir (+ (Variables|Default|GetCountJumpInAir) 1))
        (else
          (Character|Jump)
          (Variables|Default|SetCountJumpInAir (+ (Variables|Default|GetCountJumpInAir) 1)))))))

(event Input|ActionEvents|InputActionDeJump
  (params (Key :type Key%20Structure :default "None"))
  ;[1 1 1] Jump L/R
  (:Pressed
    (if (Variables|Default|GetIsInAir)
      (Physics|AddForce (Variables|Character|GetCharacterMovement) "0, 0,-6000000.000000"))))

(event Input|ActionEvents|InputActionJumpRight
  (params (Key :type Key%20Structure :default "None"))
  ;[1 1 1] Jump L/R
  (:Pressed
    (if (not (Variables|Default|GetIsDeath))
      (if (> (Variables|Default|GetCurrentLane) (* (/ (Variables|Default|GetMaxLane) 2) -1))
        (if (< (Variables|Default|GetCountJumpInAir) 2)
          (Pawn|Input|AddMovementInput (Class|PawnMovementComponent|GetPawnOwner (Variables|Character|GetCharacterMovement)) (Math|Vector|MakeVector 1.0 -1.0 0.0) 1.0 false)
          (Character|Jump)
          (Variables|Default|SetCurrentLane (- (Variables|Default|GetCurrentLane) 1))
          (Variables|Default|SetCountJumpInAir (+ (Variables|Default|GetCountJumpInAir) 1)))))))

(event Input|ActionEvents|InputActionJumpLeft
  (params (Key :type Key%20Structure :default "None"))
  ;[1 1 1] Jump L/R
  (:Pressed
    (if (not (Variables|Default|GetIsDeath))
      (if (< (Variables|Default|GetCurrentLane) (/ (Variables|Default|GetMaxLane) 2))
        (if (< (Variables|Default|GetCountJumpInAir) 2)
          (Pawn|Input|AddMovementInput (Class|PawnMovementComponent|GetPawnOwner (Variables|Character|GetCharacterMovement)) (Math|Vector|MakeVector 1.0 1.0 0.0) 1.0 false)
          (Character|Jump)
          (Variables|Default|SetCurrentLane (+ (Variables|Default|GetCurrentLane) 1))
          (Variables|Default|SetCountJumpInAir (+ (Variables|Default|GetCountJumpInAir) 1)))))))

(event Input|KeyboardEvents|AnyKey
  (params (Key :type Key%20Structure :default "None"))
  (bind _returnvalue (Game|GetPlayerCharacter 0))
  (bind _slotitemused (Variables|Default|GetSlotItemUsed))
  (bind _returnvalue_2 (Transformation|GetActorTransform _returnvalue))
  (:Pressed
    (if (or (== Key "E") (== Key "Q"))
      (if (Utilities|Array|IsNotEmpty _slotitemused)
        (if (not (Variables|Default|GetCureentCasting))
          (bind (_output _whatkey) (CallFunction|CheckKey _slotitemused Key))
          (if _whatkey
            (if (and (== (Variables|Default|GetItemObjectQ) 0) (> (.Value (Utilities|Map|Find (Variables|Default|GetPlayerItem) _output)) 0))
              (bind _returnvalue_3 (Game|SpawnActorfromClass _output _returnvalue_2 "Undefined" 0 0))
              (bind _output_get (Variables|Default|SetItemObjectQ _returnvalue_3))
              (Variables|/Game/Item/BaseUsedItem.BaseUsedItem_C|SetUsed? _output_get true)
              (Variables|Default|SetCureentCasting true)
              (bind _result (Math|Integer|DecrementInt (.Value (Utilities|Map|Find (Variables|Default|GetPlayerItem) _output)))
                (:%20%20
                  (Utilities|Map|Add (Variables|Default|GetPlayerItem) _output _result)
                  (bind _asjumper_bp (Utilities|Casting|CastToJumper_BP (Game|GetPlayerCharacter 0) :!label _label))
                  ;[1 1 1] Save Item
                  (bind _returnvalue_4 (SaveGame|DoesSaveGameExist "HighScoreData"))
                  (if _returnvalue_4
                    (bind _returnvalue_5 (SaveGame|LoadGamefromSlot "HighScoreData"))
                    (bind _output_get_2 (Variables|Default|SetSavegame _returnvalue_5))
                    (bind _asendless_save_game (Utilities|Casting|CastToEndless_SaveGame _output_get_2))
                    (Variables|/Game/Save/Endless_SaveGame.Endless_SaveGame_C|SetPlayerItem _asendless_save_game (Variables|Jumper_BP_C|GetPlayerItem _asjumper_bp))
                    (|AsyncSaveGametoSlot _asendless_save_game "HighScoreData")
                    (else
                      (bind _returnvalue_6 (SaveGame|CreateSaveGameObject "/Game/Save/Endless_SaveGame.Endless_SaveGame_C"))
                      (bind _output_get_3 (Variables|Default|SetSavegame _returnvalue_6))
                      (bind _asendless_save_game_2 (Utilities|Casting|CastToEndless_SaveGame _output_get_3))
                      (Variables|/Game/Save/Endless_SaveGame.Endless_SaveGame_C|SetPlayerItem _asendless_save_game_2 (Variables|Jumper_BP_C|GetPlayerItem _asjumper_bp))
                      (|AsyncSaveGametoSlot _asendless_save_game_2 "HighScoreData"))))))
            (elif (and (> (.Value (Utilities|Map|Find (Variables|Default|GetPlayerItem) _output)) 0) (== (Variables|Default|GetItemObjectE) 0))
              (bind _returnvalue_7 (Game|SpawnActorfromClass _output _returnvalue_2 "Undefined" 0 0))
              (bind _output_get_4 (Variables|Default|SetItemObjectE _returnvalue_7))
              (Variables|/Game/Item/BaseUsedItem.BaseUsedItem_C|SetUsed? _output_get_4 true)
              (Variables|Default|SetCureentCasting true)
              (bind _result_2 (Math|Integer|DecrementInt (.Value (Utilities|Map|Find (Variables|Default|GetPlayerItem) _output)))
                (:%20%20
                  (Utilities|Map|Add (Variables|Default|GetPlayerItem) _output _result_2)
                  (goto _label))))))))))

(fn ConstructionScript)

(fn SetPlayerDirection
  (params (MovementComp :type Movement%20Component%20Object%20Reference))
  ;[1 1 1] Rotate player to jump direction
  (if (== (.y (Variables|/Script/Engine.MovementComponent|GetVelocity MovementComp)) 0.0)
    (Pawn|Input|AddMovementInput (Class|PawnMovementComponent|GetPawnOwner (Variables|Character|GetCharacterMovement)) (Math|Vector|MakeVector 1.0 0.0 0.0) 1.0 false)
    (elif (> (.y (Variables|/Script/Engine.MovementComponent|GetVelocity MovementComp)) 0.0)
      (Pawn|Input|AddMovementInput (Class|PawnMovementComponent|GetPawnOwner (Variables|Character|GetCharacterMovement)) (Math|Vector|MakeVector 1.0 1.0 0.0) 1.0 false)
      (else
        (Pawn|Input|AddMovementInput (Class|PawnMovementComponent|GetPawnOwner (Variables|Character|GetCharacterMovement)) (Math|Vector|MakeVector 1.0 -1.0 0.0) 1.0 false)))))

(fn CheckKey
  (params (Array :type Array%20of%20Base%20Used%20Item%20Class%20References) (Key :type Key%20Structure :default "None"))
  (if (== Key "Q")
    (return (Utilities|Array|Get(acopy) Array) true)
    (elif (== Key "E")
      (return (Utilities|Array|Get(acopy) Array 1) false))))