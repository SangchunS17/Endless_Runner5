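; Enemy1 is a chaser enemy that trails player 0 along the world X axis at a set offset.
; Every Tick, MoveComponentTo drives its root toward the player's X minus PlayertoEnemyDisTance, keeping the enemy's own Y and Z.
; The Playerinterrup event cuts that distance by a fixed step, pulling the target point toward the player on each call.
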(event Custom|Player%20interrup
  (Variables|Default|SetPlayertoEnemyDisTance (- (Variables|Default|GetPlayertoEnemyDisTance) 1e+02)))

(event EventBeginPlay)

(event Collision|EventActorBeginOverlap
  (params (OtherActor :type Actor%20Object%20Reference)))

(event EventTick
  (params (DeltaSeconds :type Float%20%28single-precision%29))
  (bind _returnvalue (Transformation|GetActorLocation))
  (Components|MoveComponentTo (Variables|Default|GetDefaultSceneRoot) (Math|Vector|MakeVector (- (.x (Transformation|GetActorLocation (Game|GetPlayerCharacter 0))) (Variables|Default|GetPlayertoEnemyDisTance)) (.y _returnvalue) (.z _returnvalue)) "0, 0, 0" false false 0.2 false))

(fn ConstructionScript)